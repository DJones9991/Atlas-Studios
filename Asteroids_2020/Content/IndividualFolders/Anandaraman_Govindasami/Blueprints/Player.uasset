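; Player character Blueprint with yaw-relative forward movement, yaw turning, projectile firing and a shock action.
; Firing spawns a projectile just ahead of the actor, while shock briefly raises ShockVar and flashes Sphere1.
; Overlapping an Asteroid-tagged actor on the Hit component pulses a CameraShake flag and resets HealthDecreased.
; The health-loss and destroy-on-death logic is disconnected, so it never runs.
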(event `InputAxis|Forward`
  (params (AxisValue :type "Float (single-precision)"))
  (bind (_returnvalue_roll _returnvalue_pitch _returnvalue_yaw) (`KismetMathLibrary.BreakRotator` (`self.GetControlRotation`)))
  ;[1 1 1] Movement
  (`self.AddMovementInput` (`KismetMathLibrary.GetForwardVector` (`KismetMathLibrary.MakeRotator` 0.0 0.0 _returnvalue_yaw)) AxisValue))

(event `InputAction|FireWeapon`
  (params (Key :type "Key Structure"))
  (:`Pressed`
    (`|SpawnActorFromClass` "/Game/IndividualFolders/Anandaraman_Govindasami/Blueprints/Projectiles.Projectiles_C" (`KismetMathLibrary.MakeTransform` (+ (`SceneComponent.GetForwardVector` (`self.CapsuleComponent`)) (`self.K2_GetActorLocation`)) (`self.K2_GetActorRotation`)) "AdjustIfPossibleButAlwaysSpawn" "OverrideRootScale" null null)))

(event `InputAxis|Rotate`
  (params (AxisValue :type "Float (single-precision)"))
  ;[1 1 1] Movement
  (`self.AddControllerYawInput` AxisValue))

(event `InputAction|Shock`
  (params (Key :type "Key Structure"))
  (:`Pressed`
    (set `self.Shock_Var` true)
    (`SceneComponent.ToggleVisibility` (`self.Sphere1`) false)
    (`KismetSystemLibrary.Delay` 0.03)
    (set `self.Shock_Var` false)
    (`SceneComponent.ToggleVisibility` (`self.Sphere1`) false))
  (:`Released`
    (set `self.Shock_Var` false)))

(event `self.Hit.OnComponentBeginOverlap`
  (params (OverlappedComponent :type "PrimitiveComponent Object Reference") (OtherActor :type "Actor Object Reference") (OtherComp :type "PrimitiveComponent Object Reference") (OtherBodyIndex :type Integer) (bFromSweep :type Boolean) (SweepResult :type "HitResult Structure (by ref)"))
  ;[1 1 1] CameraShake
  (if (`self.ActorHasTag` OtherActor "Asteroid")
    (set `self.CameraShake` true)
    (`KismetSystemLibrary.Delay` 0.1)
    (set `self.CameraShake` false)
    (set `self.HealthDecreased` false)))

(fn `UserConstructionScript`)