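; Asteroid actor that projectiles destroy for 25 points on the Ship, with a chance to drop a pickup.
; Unless flagged Small or at 0.5 scale, it splits into two half-scale asteroids yawed 45 degrees either way.
; Drops come from cascading random rolls across eight pickup classes.
; Tick also destroys it, without points or drops, when the Player's ShockVar is on while inside Sphere1.
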(event `self.ReceiveTick`
  (params (DeltaSeconds :type "Float (single-precision)"))
  (bind _asplayer (cast `/Game/IndividualFolders/Anandaraman_Govindasami/Blueprints/Player` (`GameplayStatics.GetPlayerCharacter` 0)))
  (if (and (`/Game/IndividualFolders/Anandaraman_Govindasami/Blueprints/Player.Shock_Var` _asplayer) (`self.Shock`))
    (`self.K2_DestroyActor`)))

(event `self.Sphere1.OnComponentEndOverlap`
  (params (OverlappedComponent :type "PrimitiveComponent Object Reference") (OtherActor :type "Actor Object Reference") (OtherComp :type "PrimitiveComponent Object Reference") (OtherBodyIndex :type Integer))
  (if (== OtherActor "/Game/IndividualFolders/Anandaraman_Govindasami/Blueprints/Player.Player")
    (set `self.Shock` false)))

(event `self.Sphere1.OnComponentBeginOverlap`
  (params (OverlappedComponent :type "PrimitiveComponent Object Reference") (OtherActor :type "Actor Object Reference") (OtherComp :type "PrimitiveComponent Object Reference") (OtherBodyIndex :type Integer) (bFromSweep :type Boolean) (SweepResult :type "HitResult Structure (by ref)"))
  (if (== (`GameplayStatics.GetObjectClass` OtherActor) "/Game/IndividualFolders/Anandaraman_Govindasami/Blueprints/Player.Player_C")
    (set `self.Shock` true)))

(event `self.ReceiveHit`
  (params (MyComp :type "PrimitiveComponent Object Reference") (Other :type "Actor Object Reference") (OtherComp :type "PrimitiveComponent Object Reference") (bSelfMoved :type Boolean) (HitLocation :type "Vector Structure") (HitNormal :type "Vector Structure") (NormalImpulse :type "Vector Structure") (Hit :type "HitResult Structure (by ref)"))
  (cast `/Game/IndividualFolders/Dan_Jones/DJ_BP_Projectile` Other)
  (if (`self.Small`)
    (bind _asship (cast `/Game/IndividualFolders/Cameron_McCabe/Ship` (`GameplayStatics.GetPlayerPawn` 0)))
    (set `/Game/IndividualFolders/Cameron_McCabe/Ship.Current Points` (+ (`/Game/IndividualFolders/Cameron_McCabe/Ship.Current Points` _asship) 25.0) _asship)
    (`self.chooseUpgrade`)
    (`self.K2_DestroyActor`)
    (else
      (set `self.Scale` (`self.GetActorScale3D`))
      (set `self.Location` (`self.K2_GetActorLocation`))
      (set `self.Rotation` (`self.K2_GetActorRotation`))
      (`self.chooseUpgrade`)
      (`self.K2_DestroyActor`)
      (`self.SpawnSmallAsteroids`)
      (set `self.Small` true)
      (bind _asship_2 (cast `/Game/IndividualFolders/Cameron_McCabe/Ship` (`GameplayStatics.GetPlayerPawn` 0)))
      (set `/Game/IndividualFolders/Cameron_McCabe/Ship.Current Points` (+ (`/Game/IndividualFolders/Cameron_McCabe/Ship.Current Points` _asship_2) 25.0) _asship_2))))

(event `chooseUpgrade`
  (bind _returnvalue (`KismetMathLibrary.RandomInteger` 99))
  ;[1 1 1] Ethan's Work
  (if (< _returnvalue 11)
    (set `self.spawnedUpgrade` "/Game/IndividualFolders/Lewis_Clark/LC_BP_DisableThrustersPickup.LC_BP_DisableThrustersPickup_C")
    (`self.spawnUpgrade` :!label _label)
    (elif (< _returnvalue 22)
      (set `self.spawnedUpgrade` "/Game/IndividualFolders/Lewis_Clark/LC_BP_DisableWeaponsPickup.LC_BP_DisableWeaponsPickup_C")
      (goto _label)
      (elif (< _returnvalue 33)
        (set `self.spawnedUpgrade` "/Game/IndividualFolders/Lewis_Clark/LC_BP_DoublePointsPickup.LC_BP_DoublePointsPickup_C")
        (goto _label)
        (elif (< _returnvalue 44)
          (set `self.spawnedUpgrade` "/Game/IndividualFolders/Lewis_Clark/LC_BP_HealthRegenPickup.LC_BP_HealthRegenPickup_C")
          (goto _label)
          (elif (< _returnvalue 55)
            (set `self.spawnedUpgrade` "/Game/IndividualFolders/Lewis_Clark/LC_BP_PointsPickup.LC_BP_PointsPickup_C")
            (goto _label)
            (elif (< _returnvalue 66)
              (set `self.spawnedUpgrade` "/Game/IndividualFolders/Lewis_Clark/LC_BP_ShieldPickup.LC_BP_ShieldPickup_C")
              (goto _label)
              (elif (< _returnvalue 77)
                (set `self.spawnedUpgrade` "/Game/IndividualFolders/Lewis_Clark/LC_BP_SlowDownPickup.LC_BP_SlowDownPickup_C")
                (goto _label)
                (elif (< _returnvalue 88)
                  (set `self.spawnedUpgrade` "/Game/IndividualFolders/Lewis_Clark/LC_BP_SpeedBoostPickup.LC_BP_SpeedBoostPickup_C")
                  (goto _label))))))))))

(event `spawnUpgrade`
  ;[1 1 1] Ethan's Work
  (`|SpawnActorFromClass` (`self.spawnedUpgrade`) (`self.GetTransform`) "AlwaysSpawn" "OverrideRootScale" null null))

(fn `SpawnSmallAsteroids`
  (bind (_rotation_roll _rotation_pitch _rotation_yaw) (`KismetMathLibrary.BreakRotator` (`self.Rotation`)))
  (if (!= (- (`self.Scale`) (0.5 0.5 0.5)) (0.0 0.0 0.0))
    (`|SpawnActorFromClass` "Asteroid_C" (`KismetMathLibrary.MakeTransform` (`self.Location`) (`KismetMathLibrary.MakeRotator` _rotation_roll _rotation_pitch (+ _rotation_yaw 45.0)) (/ (`self.Scale`) (2.0 2.0 2.0))) "Undefined" "OverrideRootScale" null null)
    (`|SpawnActorFromClass` "Asteroid_C" (`KismetMathLibrary.MakeTransform` (`self.Location`) (`KismetMathLibrary.MakeRotator` 0.0 0.0 (- _rotation_yaw 45.0)) (/ (`self.Scale`) (2.0 2.0 2.0))) "Undefined" "OverrideRootScale" null null)))

(fn `UserConstructionScript`)